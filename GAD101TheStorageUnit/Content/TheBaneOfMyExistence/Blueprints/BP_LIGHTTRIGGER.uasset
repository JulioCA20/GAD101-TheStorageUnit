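; BP_LIGHTTRIGGER is a trigger volume that switches a rect light with box overlaps.
; Any actor entering the box sets the light to a bright fixed intensity, but only the player character sets the ActivatedByPlayer flag.
; Any exit restarts a timeline that drives the intensity.
; A Delay on the timeline's Update pin later prints "Light Off" and clears the flag.
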(event `self.Box.OnComponentBeginOverlap`
  (params (OverlappedComponent :type "PrimitiveComponent Object Reference") (OtherActor :type "Actor Object Reference") (OtherComp :type "PrimitiveComponent Object Reference") (OtherBodyIndex :type Integer) (bFromSweep :type Boolean) (SweepResult :type "HitResult Structure (by ref)"))
  (`LightComponent.SetIntensity` (`self.RectLight`) 8000.0)
  (if (== OtherActor (`GameplayStatics.GetPlayerCharacter` 0))
    (set `self.bActivatedByPlayer` true)))

(event `self.Box.OnComponentEndOverlap`
  (params (OverlappedComponent :type "PrimitiveComponent Object Reference") (OtherActor :type "Actor Object Reference") (OtherComp :type "PrimitiveComponent Object Reference") (OtherBodyIndex :type Integer))
  (bind (_direction _newtrack_0) (`Timeline|Timeline` :!via `PlayFromStart`)
    (:`Update`
      (`LightComponent.SetIntensity` (`self.RectLight`) _newtrack_0)
      (`KismetSystemLibrary.Delay` 15.0)
      (`KismetSystemLibrary.PrintString` "Light Off")
      (set `self.bActivatedByPlayer` false))))

(fn `UserConstructionScript`)