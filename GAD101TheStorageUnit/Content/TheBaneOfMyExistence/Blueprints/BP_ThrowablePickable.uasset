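; BP_ThrowablePickable is an interactable pickup actor, apparently for a throwable bottle.
; An interaction request through its Blueprint interface fires PickUp, which sends a pickup message to player 0's character.
; It then casts to BP_FirstPersonCharacter and destroys itself only if that character's BPickUpBottle flag is set.
; The interaction request always returns false, and the retrieve-item interface function is an empty stub.
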(event `PickUp`
  (bind _returnvalue (`GameplayStatics.GetPlayerCharacter` 0))
  (message `/Game/Input/BlueprintInterfaces/BPI_Player.BPI_Pickup` _returnvalue)
  (bind _asbp_first_person_character (cast `/Game/FirstPerson/Blueprints/BP_FirstPersonCharacter` _returnvalue))
  (if (`/Game/FirstPerson/Blueprints/BP_FirstPersonCharacter.B_PickUpBottle?` _asbp_first_person_character)
    (`self.K2_DestroyActor`)))

(fn `BPI_InteractionRequest`
  (returns (Success :type Boolean))
  (`self.PickUp`)
  (return false))

(fn `BPI_RetrieveItem`
  (returns (BP_ITEM :type "/Game/INVENTORY/BLUEPRINTS/InteractableItems/BP_ITEM Object Reference"))
  (return null))

(fn `UserConstructionScript`)