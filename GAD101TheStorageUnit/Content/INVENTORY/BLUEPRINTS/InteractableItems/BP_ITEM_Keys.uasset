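; BP_ITEM_Keys is an interactable key pickup for the inventory system.
; On interaction request it plays a key sound and passes its KeyID to the player character through an add-key interface message.
; If the player accepts the key, the actor destroys itself and returns the result.
; The event graph holds only disabled default events, so all logic lives in the interaction interface function.
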(fn `BPI_InteractionRequest`
  (returns (Success :type Boolean))
  (`GameplayStatics.PlaySound2D` "/Game/Audio/keys.keys" 1.0 1.0 0.0 null null)
  (bind _success (message `/Game/Input/BlueprintInterfaces/BPI_Player.BPI_AddKeyRequest` (`GameplayStatics.GetPlayerCharacter` 0) (`self.KeyID`)))
  (if _success
    (`self.K2_DestroyActor`)
    (return _success)))

(fn `UserConstructionScript`
  (`parent.UserConstructionScript`))