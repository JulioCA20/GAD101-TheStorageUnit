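; BP_ITEM is an interactable world item that shows an icon when the player comes near.
; The construction script applies the Item's mesh with physics off.
; Outer-sphere overlaps toggle the outer icon for the player character; inner-sphere events are empty, and the interaction interface request just returns false.
; A separate sphere-construction function sizes collisions, places icons, scales the mesh and sets debug icon visibility, but no shown graph calls it.
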(event `self.B_innercollision.OnComponentBeginOverlap`
  (params (OverlappedComponent :type "PrimitiveComponent Object Reference") (OtherActor :type "Actor Object Reference") (OtherComp :type "PrimitiveComponent Object Reference") (OtherBodyIndex :type Integer) (bFromSweep :type Boolean) (SweepResult :type "HitResult Structure (by ref)")))

(event `self.B_innercollision.OnComponentEndOverlap`
  (params (OverlappedComponent :type "PrimitiveComponent Object Reference") (OtherActor :type "Actor Object Reference") (OtherComp :type "PrimitiveComponent Object Reference") (OtherBodyIndex :type Integer)))

(event `self.A_outercollision.OnComponentBeginOverlap`
  (params (OverlappedComponent :type "PrimitiveComponent Object Reference") (OtherActor :type "Actor Object Reference") (OtherComp :type "PrimitiveComponent Object Reference") (OtherBodyIndex :type Integer) (bFromSweep :type Boolean) (SweepResult :type "HitResult Structure (by ref)"))
  (if (== OtherActor (`GameplayStatics.GetPlayerCharacter` 0))
    (`SceneComponent.SetVisibility` (`self.outer_icon`) true false)))

(event `self.A_outercollision.OnComponentEndOverlap`
  (params (OverlappedComponent :type "PrimitiveComponent Object Reference") (OtherActor :type "Actor Object Reference") (OtherComp :type "PrimitiveComponent Object Reference") (OtherBodyIndex :type Integer))
  (if (== (`GameplayStatics.GetPlayerCharacter` 0) OtherActor)
    (`SceneComponent.SetVisibility` (`self.outer_icon`) false false)))

(fn `BPI_InteractionRequest`
  (returns (Success :type Boolean))
  (return false))

(fn `Construction for sphere`
  (bind _staticmesh (`self.StaticMesh`))
  (`|ExecutionSequence`
    (:`then_0`
      ; setting radius for collisions
      ;; probs dont need this but yet to see
      (`SphereComponent.SetSphereRadius` (`self.B_innercollision`) (`self.InnerSphereRadius`) true)
      (`SphereComponent.SetSphereRadius` (`self.A_outercollision`) (`self.OuterSphereRadius`) true)
      ; setting location of icons
      (`SceneComponent.K2_SetRelativeLocation` (`self.inner_icon`) (`self.Icon Location`) false false)
      (`SceneComponent.K2_SetRelativeLocation` (`self.outer_icon`) (`self.Icon Location`) false false))
    (:`then_1`
      (`StaticMeshComponent.SetStaticMesh` (`self.StaticMesh`) (`self.item_mesh`))
      (`SceneComponent.K2_SetWorldTransform` _staticmesh (`KismetMathLibrary.MakeTransform` (`SceneComponent.K2_GetComponentLocation` _staticmesh) (`SceneComponent.K2_GetComponentRotation` _staticmesh) (`self.Item Scale`)) false false))
    (:`then_2`
      (if (`self.debugging`)
        (`SceneComponent.SetVisibility` (`self.inner_icon`) true false)
        (`SceneComponent.SetVisibility` (`self.outer_icon`) true false)
        (else
          (`SceneComponent.SetVisibility` (`self.inner_icon`) false false)
          (`SceneComponent.SetVisibility` (`self.outer_icon`) false false))))))

(fn `UserConstructionScript`
  (bind _staticmesh (`self.StaticMesh`))
  (`StaticMeshComponent.SetStaticMesh` _staticmesh (`.Mesh_14_AC16F17A465C128306F5D08A843F9276` (break `/Game/INVENTORY/BLUEPRINTS/S_ITEM_STRUCTURE` (`self.item`))))
  (`PrimitiveComponent.SetSimulatePhysics` _staticmesh false))