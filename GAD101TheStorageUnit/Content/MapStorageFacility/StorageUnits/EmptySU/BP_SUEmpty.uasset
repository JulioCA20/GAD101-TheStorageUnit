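; BP_SUEmpty is an empty storage unit with a lockable door that slides up and down.
; An interaction request toggles the door, or, when it is locked, asks the player character for the matching KeyID through an interface and only unlocks it.
; MoveComponentTo animates the door, with an InProgress flag meant to block overlapping moves.
; Ending overlap with the Box closes the door after a short delay.
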(event `UnlockDoor`
  ; Locks Door or Unlocks
  (set `self.Locked` false))

(event `ToggleDoor`
  ; Close or Open the door accordingly to the open boolean
  (if (`self.Open`)
    (`self.CloseDoor`)
    (else
      (`self.OpenDoor`))))

(event `OpenDoor`
  (if (not (`self.InProgress?`))
    (set `self.InProgress?` true)
    (`KismetSystemLibrary.MoveComponentTo` (`self.Door`) (0.0 272.0 245.0) (struct) false true 1.0)
    (set `self.Open` true)
    (set `self.InProgress?` false)))

(event `self.Box.OnComponentEndOverlap`
  (params (OverlappedComponent :type "PrimitiveComponent Object Reference") (OtherActor :type "Actor Object Reference") (OtherComp :type "PrimitiveComponent Object Reference") (OtherBodyIndex :type Integer))
  (`KismetSystemLibrary.Delay` 0.5)
  (`self.CloseDoor`))

(event `CloseDoor`
  (if (not (`self.InProgress?`))
    (set `self.InProgress?` true)
    (`KismetSystemLibrary.MoveComponentTo` (`self.Door`) (0.0 272.0 0.0) (struct) true true 1.0)
    (set `self.Open` false)
    (set `self.InProgress?` false)))

(fn `BPI_InteractionRequest`
  (returns (Success :type Boolean))
  (`self.LockCheck`)
  (return false))

(fn `LockCheck`
  (if (`self.Locked`)
    (bind _success (message `/Game/Input/BlueprintInterfaces/BPI_Player.BPI_KeyRequest` (`GameplayStatics.GetPlayerCharacter` 0) (`self.KeyID`)))
    (if _success
      (`self.UnlockDoor`))
    (else
      (`self.ToggleDoor`))))

(fn `UserConstructionScript`)