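; BP_LIGHTForunit is a proximity-triggered light for storage units, built from a Box trigger and a RectLight.
; Any overlap raises the light intensity, as the player-character check follows that change and leads nowhere.
; Ending an overlap zeroes the intensity immediately, then after a delay prints "Light Off" and clears ActivatedByPlayer, which these graphs never set true.
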(event `self.Box.OnComponentBeginOverlap`
  (params (OverlappedComponent :type "PrimitiveComponent Object Reference") (OtherActor :type "Actor Object Reference") (OtherComp :type "PrimitiveComponent Object Reference") (OtherBodyIndex :type Integer) (bFromSweep :type Boolean) (SweepResult :type "HitResult Structure (by ref)"))
  (`LightComponent.SetIntensity` (`self.RectLight`) 8000.0)
  (if (== OtherActor (`GameplayStatics.GetPlayerCharacter` 0))
    _))

(event `self.Box.OnComponentEndOverlap`
  (params (OverlappedComponent :type "PrimitiveComponent Object Reference") (OtherActor :type "Actor Object Reference") (OtherComp :type "PrimitiveComponent Object Reference") (OtherBodyIndex :type Integer))
  (`LightComponent.SetIntensity` (`self.RectLight`) 0.0)
  (`KismetSystemLibrary.Delay` 15.0)
  (`KismetSystemLibrary.PrintString` "Light Off")
  (set `self.bActivatedByPlayer` false))

(fn `UserConstructionScript`)