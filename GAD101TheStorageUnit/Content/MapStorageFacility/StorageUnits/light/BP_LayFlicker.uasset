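; BP_LayFlicker is a flickering point light actor for the storage units in the storage facility map.
; The construction script applies a base Intensity to the PointLight.
; From BeginPlay, a looping retriggerable delay waits a random time between Min and Max, then a FlipFlop alternates the light between MinFlicker and MaxFlicker intensities.
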(event `self.ReceiveBeginPlay`
  (bind _pointlight (`self.PointLight`))
  (`KismetSystemLibrary.RetriggerableDelay` (`KismetMathLibrary.RandomFloatInRange` (`self.Min`) (`self.Max`)) :!label _label)
  (`/Engine/EditorBlueprintResources/StandardMacros.FlipFlop`
    (:`A`
      (`LightComponent.SetIntensity` _pointlight (`self.Min flicker`))
      (goto _label))
    (:`B`
      (`LightComponent.SetIntensity` _pointlight (`self.Max Flicker`))
      (goto _label))))

(fn `UserConstructionScript`
  (`LightComponent.SetIntensity` (`self.PointLight`) (`self.intensity`)))