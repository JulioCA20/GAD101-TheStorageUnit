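; BP_Booleen is a generated dynamic mesh actor in the storage unit base wall set that builds a resizable box, likely a boolean volume for walls.
; On rebuild, Geometry Script resets the mesh and appends a centered box sized at twice the Position vector, which acts as half-extents.
; The construction script matches the Box component's extent to Position and sets mesh material slot zero with no material specified.
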(event `self.OnRebuildGeneratedMesh`
  (params (TargetMesh :type "DynamicMesh Object Reference"))
  (bind (_position_x _position_y _position_z) (`KismetMathLibrary.BreakVector` (`self.Position`)))
  (bind _returnvalue (`DynamicMesh.Reset` TargetMesh))
  (`GeometryScriptLibrary_MeshPrimitiveFunctions.AppendBox` _returnvalue (struct) (struct) (* _position_x 2.0) (* _position_y 2.0) (* _position_z 2.0) 0 0 0 "Center"))

(fn `UserConstructionScript`
  (`PrimitiveComponent.SetMaterial` (`self.DynamicMeshComponent`) 0 null)
  (`BoxComponent.SetBoxExtent` (`self.Box`) (`self.Position`) true))