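; BP_BaseWall is a generated dynamic-mesh actor that builds a box wall with cutouts using Geometry Script.
; On rebuild, it resets the mesh, appends a box sized by PositionofWall, then boolean-subtracts each listed DynamicMeshActor's mesh, aligned by actor transforms.
; The construction script applies the wall material.
; CoventToStaticMesh bakes the result into a new static mesh asset, but sets its material only on the Failure branch.
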(event `self.OnRebuildGeneratedMesh`
  (params (TargetMesh :type "DynamicMesh Object Reference"))
  (`self.UpdataMeshofWall`))

(fn `coventToStaticMesh`
  (bind _returnvalue (`BaseDynamicMeshComponent.GetDynamicMesh` (`self.DynamicMeshComponent`)))
  (bind _returnvalue_2 (`GeometryScriptLibrary_CreateNewAssetFunctions.CreateNewStaticMeshAssetFromMesh` _returnvalue (`KismetStringLibrary.Concat_StrStr` (`self.NewPath`) (`self.NewName`)))
    (:`Failure`
      (`StaticMesh.SetMaterial` _returnvalue_2 0 (`self.Material`)))))

(fn `UpdataMeshofWall`
  (locals (NewLocalVar :type "Vector Structure" :default (0.0 0.0 0.0)))
  (bind (_positionofwall_x _positionofwall_y _positionofwall_z) (`KismetMathLibrary.BreakVector` (`self.PositionofWall`)))
  (bind _returnvalue (`BaseDynamicMeshComponent.GetDynamicMesh` (`self.DynamicMeshComponent`)))
  (bind _returnvalue_2 (`DynamicMesh.Reset` _returnvalue))
  (bind _returnvalue_3 (`GeometryScriptLibrary_MeshPrimitiveFunctions.AppendBox` _returnvalue_2 (struct) (`KismetMathLibrary.MakeTransform` (`KismetMathLibrary.MakeVector` (/ _positionofwall_x 2.0) (/ _positionofwall_y 2.0))) _positionofwall_x _positionofwall_y _positionofwall_z))
  (for _array_element (`self.Actor`)
    (bind _asdynamic_mesh_actor (cast `DynamicMeshActor` _array_element))
    (bind _returnvalue_4 (`BaseDynamicMeshComponent.GetDynamicMesh` (`DynamicMeshActor.DynamicMeshComponent` _asdynamic_mesh_actor)))
    (bind _alignmenttransform (`ARBlueprintLibrary.CalculateAlignmentTransform` (`self.GetTransform` self) (`self.GetTransform` _array_element)))
    (`GeometryScriptLibrary_MeshBooleanFunctions.ApplyMeshBoolean` _returnvalue_3 (struct) _returnvalue_4 _alignmenttransform "Subtract")))

(fn `UserConstructionScript`
  (`PrimitiveComponent.SetMaterial` (`self.DynamicMeshComponent`) 0 (`self.Material`)))